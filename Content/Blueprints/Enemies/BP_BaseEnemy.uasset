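; BP_BaseEnemy is a base enemy actor that travels along a spline path placed in the level.
; On BeginPlay it finds all BP_Spline actors and keeps the first as its path.
; Each Tick it adds Speed times delta time to a running distance, then snaps its transform to that point on the spline in world space.
; The graph has no end-of-path handling.
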(event `self.ReceiveBeginPlay`
  (bind _outactors (`GameplayStatics.GetAllActorsOfClass` "/Game/Blueprints/WorldElements/BP_Spline.BP_Spline_C"))
  (bind _output_get (set `self.Splines` _outactors))
  (set `self.Spline` (`|GetArrayItem` _output_get)))

(event `self.ReceiveTick`
  (params (DeltaSeconds :type "Float (single-precision)"))
  (bind (_returnvalue_location _returnvalue_rotation _returnvalue_scale) (`KismetMathLibrary.BreakTransform` (`SplineComponent.GetTransformAtDistanceAlongSpline` (`/Game/Blueprints/WorldElements/BP_Spline.Spline` (`self.Spline`)) (`self.CurrentDistanceBySpline`) "World" false)))
  (set `self.CurrentDistanceBySpline` (+ (* DeltaSeconds (`self.Speed`)) (`self.CurrentDistanceBySpline`)))
  (`self.K2_SetActorTransform` (`KismetMathLibrary.MakeTransform` _returnvalue_location _returnvalue_rotation _returnvalue_scale)))

(fn `UserConstructionScript`)